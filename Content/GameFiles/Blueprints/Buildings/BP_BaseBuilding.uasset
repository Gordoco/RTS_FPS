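; Base building Blueprint that handles fog-of-war reveal for buildings on the player's team.
; On BeginPlay it compares the player controller's Team to its own, then sets MapRevealer to permanent and caches the first MapFog actor.
; The RTS_FPSController lookup tries player ID 0 first and falls back to player index 0 if the cast fails; an unwired debug print labels that failure as Steam-only.
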(event `self.ReceiveBeginPlay`
  (bind _asrts_fpscontroller (cast `/Game/GameFiles/Blueprints/Players/Controllers/RTS_FPSController` (`GameplayStatics.GetPlayerControllerFromID` 0))
    (:`then`
      (if (== (`RTSPlayerController.Team` _asrts_fpscontroller) (`self.Team`))
        (`MapRevealerComponent.SetRevealMode` (`self.MapRevealer`) "Permanent")
        (bind _outactors (`GameplayStatics.GetAllActorsOfClass` "/Script/MinimapPlugin.MapFog"))
        (set `self.FogActor` (`|GetArrayItem` _outactors))))
    (:`CastFailed`
      (bind _asrts_fpscontroller_2 (cast `/Game/GameFiles/Blueprints/Players/Controllers/RTS_FPSController` (`GameplayStatics.GetPlayerController` 0)))
      (if (== (`RTSPlayerController.Team` _asrts_fpscontroller_2) (`self.Team`))
        (`MapRevealerComponent.SetRevealMode` (`self.MapRevealer`) "Permanent")
        (bind _outactors_2 (`GameplayStatics.GetAllActorsOfClass` "/Script/MinimapPlugin.MapFog"))
        (set `self.FogActor` (`|GetArrayItem` _outactors_2))))))

(fn `UserConstructionScript`)