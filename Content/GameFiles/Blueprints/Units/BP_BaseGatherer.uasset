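; BP_BaseGatherer is an RTS gatherer unit with team-colored trooper visuals, a resource bar and minimap presence.
; BeginPlay sets materials and icon color by team, then enables fog revealing if the local player controller's team matches, with a fallback lookup for a Steam cast failure.
; Events update the multicast resource bar and debug action label, play death visuals, and fire spread-randomized projectiles with muzzle effects.
; Construction sizes the revealer from VisionRange.
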(event `self.BP_SwappedActions`
  (if (`SceneComponent.bVisible` (`self.DEBUG_Actions`))
    (bind _asdebug_action_tracker (cast `/Game/GameFiles/Blueprints/Units/DEBUG_ActionTracker` (`WidgetComponent.GetWidget` (`self.DEBUG_Actions`))))
    (set `/Game/GameFiles/Blueprints/Units/DEBUG_ActionTracker.DebugMessage` (`KismetTextLibrary.Conv_StringToText` (`.Action_Type` (break `Action` (`self.CurrentAction`)))) _asdebug_action_tracker)))

(event `MULTICAST_UpdateResources`
  (bind _resourcebar (`self.ResourceBar`))
  (if (== (`self.GetResources`) 0.0)
    (`SceneComponent.SetVisibility` _resourcebar false false)
    (else
      (`SceneComponent.SetVisibility` _resourcebar true false)
      (bind _asresource_bar (cast `/Game/GameFiles/UserInterface/Widgets/ResourceBar` (`WidgetComponent.GetWidget` (`self.ResourceBar`))))
      (set `/Game/GameFiles/UserInterface/Widgets/ResourceBar.ResourcePercent` (/ (`self.GetResources`) (`self.MaxResources`)) _asresource_bar))))

(event `self.BP_UpdateResourceCounter`
  (`self.MULTICAST_UpdateResources`))

(event `self.ReceiveBeginPlay`
  (bind _team (`self.Team`))
  (bind _mesh (`self.Mesh`))
  (switch `int` (`self.Team`)
    (:`Default`
      _)
    (:`0`
      (`PrimitiveComponent.SetMaterial` _mesh 6 "/Game/StylizedArmoredTrooper/Materials/MI_trooper_arms_default.MI_trooper_arms_default")
      (`PrimitiveComponent.SetMaterial` _mesh 7 "/Game/StylizedArmoredTrooper/Materials/MI_trooper_legs_default.MI_trooper_legs_default")
      (`PrimitiveComponent.SetMaterial` _mesh 4 "/Game/StylizedArmoredTrooper/Materials/MI_trooper_helm_default.MI_trooper_helm_default")
      (`PrimitiveComponent.SetMaterial` _mesh 5 "/Game/StylizedArmoredTrooper/Materials/MI_trooper_armor_default.MI_trooper_armor_default")
      (`MapIconComponent.SetIconDrawColor` (`self.MapIcon`) (`KismetMathLibrary.MakeColor` 1.0)))
    (:`1`
      (`PrimitiveComponent.SetMaterial` _mesh 4 "/Game/StylizedArmoredTrooper/Materials/MI_trooper_helm_green.MI_trooper_helm_green")
      (`PrimitiveComponent.SetMaterial` _mesh 5 "/Game/StylizedArmoredTrooper/Materials/MI_trooper_armor_green.MI_trooper_armor_green")
      (`PrimitiveComponent.SetMaterial` _mesh 6 "/Game/StylizedArmoredTrooper/Materials/MI_trooper_arms_green.MI_trooper_arms_green")
      (`PrimitiveComponent.SetMaterial` _mesh 7 "/Game/StylizedArmoredTrooper/Materials/MI_trooper_legs_green.MI_trooper_legs_green")
      (`MapIconComponent.SetIconDrawColor` (`self.MapIcon`) (`KismetMathLibrary.MakeColor` 0.0 1.0))))
  (bind _asrts_fpscontroller (cast `/Game/GameFiles/Blueprints/Players/Controllers/RTS_FPSController` (`GameplayStatics.GetPlayerControllerFromID` 0))
    (:`then`
      (bind _team_2 (`RTSPlayerController.Team` _asrts_fpscontroller))
      (if (== _team_2 _team)
        (`KismetSystemLibrary.PrintString` (`KismetStringLibrary.Concat_StrStr` "PC Team: " (`KismetStringLibrary.Conv_IntToString` _team_2) "UNIT TEAM: " (`KismetStringLibrary.Conv_IntToString` _team)))
        (`MapRevealerComponent.SetRevealMode` (`self.MapRevealer`) "Permanent")
        (bind _outactors (`GameplayStatics.GetAllActorsOfClass` "/Script/MinimapPlugin.MapFog"))
        (set `self.FogActor` (`|GetArrayItem` _outactors))
        (else
          (`KismetSystemLibrary.PrintString` "NOT TEAMED"))))
    (:`CastFailed`
      (`KismetSystemLibrary.PrintString` "STRANGE STEAM ONLY CAST FAIL")
      (bind _asrts_fpscontroller_2 (cast `/Game/GameFiles/Blueprints/Players/Controllers/RTS_FPSController` (`GameplayStatics.GetPlayerController` 0))
        (:`then`
          (if (== (`RTSPlayerController.Team` _asrts_fpscontroller_2) (`self.Team`))
            (`MapRevealerComponent.SetRevealMode` (`self.MapRevealer`) "Permanent")
            (bind _outactors_2 (`GameplayStatics.GetAllActorsOfClass` "/Script/MinimapPlugin.MapFog"))
            (set `self.FogActor` (`|GetArrayItem` _outactors_2))
            (else
              (`KismetSystemLibrary.PrintString` "NOT TEAMED"))))
        (:`CastFailed`
          (`KismetSystemLibrary.PrintString` "Second Cast Fail"))))))

(event `self.BP_Die_Visuals`
  (`SkeletalMeshComponent.PlayAnimation` (`self.Mesh`) "/Game/StylizedArmoredTrooper/Demo/Mannequin/Animations/TrooperDefaultDeath.TrooperDefaultDeath" false)
  (`MapIconComponent.SetIconVisible` (`self.MapIcon`) false)
  (`MapRevealerComponent.SetRevealMode` (`self.MapRevealer`) "Off"))

(event `AddParticleEffect`
  (bind (_returnvalue_roll _returnvalue_pitch _returnvalue_yaw) (`KismetMathLibrary.BreakRotator` (`self.K2_GetActorRotation`)))
  (bind _curr (`self.Curr`))
  (bind _returnvalue (`SceneComponent.GetSocketLocation` (`self.Mesh`) "socket_Rifle_Muzzle"))
  (`/Engine/EditorBlueprintResources/StandardMacros.IsValid` _curr
    (:`Is Valid`
      (`ActorComponent.K2_DestroyComponent` _curr))
    (:`Is Not Valid`
      _))
  (bind _returnvalue_2 (`GameplayStatics.SpawnEmitterAtLocation` "/Game/StylizedArmoredTrooper/Particles/P_MuzzleFlash.P_MuzzleFlash" _returnvalue (`self.K2_GetActorRotation`) (0.3 0.3 0.3)))
  (set `self.Curr` _returnvalue_2)
  (bind _returnvalue_3 (`|SpawnActorFromClass` "/Game/StylizedArmoredTrooper/Demo/Blueprints/BP_Projectile.BP_Projectile_C" (`KismetMathLibrary.MakeTransform` _returnvalue (`KismetMathLibrary.MakeRotator` (+ _returnvalue_roll (`KismetMathLibrary.RandomFloatInRange` -2.0 2.0)) (+ (`KismetMathLibrary.RandomFloatInRange` -2.0 2.0) _returnvalue_pitch) (+ _returnvalue_yaw (`KismetMathLibrary.RandomFloatInRange` -2.0 2.0)))) "AlwaysSpawn" "OverrideRootScale" null self))
  (`self.SetActorTickEnabled` _returnvalue_3 false)
  (`GameplayStatics.PlaySoundAtLocation` "/Game/StylizedArmoredTrooper/Sounds/Cue/Cue_PlasmaShot_02.Cue_PlasmaShot_02" _returnvalue (struct) 1.0 1.0 0.0 null null null null))

(fn `UserConstructionScript`
  (bind _visionrange (`self.VisionRange`))
  (`BoxComponent.SetBoxExtent` (`self.MapRevealer`) (`KismetMathLibrary.MakeVector` _visionrange _visionrange) true))