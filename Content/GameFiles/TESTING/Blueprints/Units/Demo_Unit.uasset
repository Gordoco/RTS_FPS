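; Demo_Unit is a team-based unit Blueprint that extends its parent's death handling for conquest objectives and building ownership.
; When DieVisuals fires, it runs the parent logic, then scans every ConquestObj actor and removes itself from the overlapped-unit array matching its team (0 or 1).
; It then notifies its OwningBuilding, if valid, that the unit died.
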(event `self.BP_Die_Visuals`
  (bind _owningbuilding (`self.OwningBuilding`))
  (`parent.BP_Die_Visuals`)
  (`self.RemoveFromAllConquestObjs`)
  (`/Engine/EditorBlueprintResources/StandardMacros.IsValid` _owningbuilding
    (:`Is Valid`
      (`/Game/GameFiles/TESTING/Blueprints/Buildings/Demo_UnitSpawner.UnitDied` _owningbuilding))))

(event `RemoveFromAllConquestObjs`
  (bind _outactors (`GameplayStatics.GetAllActorsOfClass` "/Game/GameFiles/TESTING/Blueprints/Misc/ConquestObj.ConquestObj_C"))
  (for _array_element _outactors
    (switch `int` (`self.Team`)
      (:`0`
        (bind _overlappedt1units (`/Game/GameFiles/TESTING/Blueprints/Misc/ConquestObj.OverlappedT1Units` _array_element))
        (bind _returnvalue (`KismetArrayLibrary.Array_Find` _overlappedt1units self))
        (if (!= _returnvalue -1)
          (`KismetArrayLibrary.Array_Remove` _overlappedt1units _returnvalue)))
      (:`1`
        (bind _overlappedt2units (`/Game/GameFiles/TESTING/Blueprints/Misc/ConquestObj.OverlappedT2Units` _array_element))
        (bind _returnvalue_2 (`KismetArrayLibrary.Array_Find` _overlappedt2units self))
        (if (!= _returnvalue_2 -1)
          (`KismetArrayLibrary.Array_Remove` _overlappedt2units _returnvalue_2))))))

(fn `UserConstructionScript`
  (`parent.UserConstructionScript`))