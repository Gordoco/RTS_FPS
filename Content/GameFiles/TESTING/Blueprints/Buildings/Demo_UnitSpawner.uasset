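; Demo unit spawner building that keeps spawning Demo_Unit actors for its team up to a population cap.
; While active, the authority runs a self-looping delay timer, begun shortly after BeginPlay or via Start.
; Each unit spawns above the building, receives its owner, team and default controller, then gets a move action to the rally point.
; The UnitDied event decrements the live count, freeing a slot for the next spawn.
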(event `UnitDied`
  (`/Engine/EditorBlueprintResources/StandardMacros.DecrementInt` (`self.CURRENTUNITS`)))

(event `self.ReceiveBeginPlay`
  (`KismetSystemLibrary.Delay` 1.0)
  (`/Engine/EditorBlueprintResources/ActorMacros.Switch Has Authority` :!label _label
    (:`Authority`
      (if (`self.bActive`)
        (`self.SpawnUnitsTimer`)))))

(event `Start`
  (goto _label))

(event `SpawnUnitsTimer`
  (if (`self.bActive`) :!label _label_2
    (if (< (`self.CURRENTUNITS`) (`self.MAXUNITS`))
      (bind _returnvalue (`|SpawnActorFromClass` "/Game/GameFiles/TESTING/Blueprints/Units/Demo_Unit.Demo_Unit_C" (`KismetMathLibrary.MakeTransform` (+ (`self.K2_GetActorLocation`) (0.0 0.0 200.0))) "AdjustIfPossibleButAlwaysSpawn" "OverrideRootScale" null self (`self.GetTeam`) null))
      (`Pawn.SpawnDefaultController` _returnvalue)
      (`BaseUnit.AddMovementAction` _returnvalue (`self.GetRallyPoint`) 0 50.0)
      (`/Engine/EditorBlueprintResources/StandardMacros.IncrementInt` (`self.CURRENTUNITS`)
        (:`  `
          _)))
    (`KismetSystemLibrary.Delay` (`self.UnitSpawnTiming`))
    (goto _label_2)))

(fn `UserConstructionScript`)