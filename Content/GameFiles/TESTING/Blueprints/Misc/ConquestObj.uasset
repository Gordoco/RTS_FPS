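; Conquest objective that two teams capture with units inside its control zone, recoloring a flag and handing over a linked building.
; On the server, overlaps track units per team: the first to enter claims a neutral point, and Tick flips it when the opposing team outnumbers the owner.
; Capture sets the building's team and, if inactive, activates it and starts unit spawning.
; An OnRep for Team refreshes the flag material.
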(event `SetFlagColor`
  (bind _team (`self.Team`))
  (bind _flag_part2 (`self.Flag_Part2`))
  (if (== _team -1)
    (`PrimitiveComponent.SetMaterial` _flag_part2 0 "/Game/GameFiles/TESTING/Models/defaultMat.defaultMat")
    (else
      (switch `int` _team
        (:`0`
          (`PrimitiveComponent.SetMaterial` _flag_part2 0 "/Game/GameFiles/TESTING/Materials/T1_Flag.T1_Flag"))
        (:`1`
          (`PrimitiveComponent.SetMaterial` _flag_part2 0 "/Game/GameFiles/TESTING/Materials/T2_Flag.T2_Flag"))))))

(event `CheckTeam1`
  (if (> (`KismetArrayLibrary.Array_Length` (`self.OverlappedT2Units`)) (`KismetArrayLibrary.Array_Length` (`self.OverlappedT1Units`)))
    (set `self.Team` 1)
    (`self.SetFlagColor`)
    (`self.CheckOwnedBuilding` 1)))

(event `self.ReceiveBeginPlay`
  (`self.SetFlagColor`))

(event `CheckTeam2`
  (if (> (`KismetArrayLibrary.Array_Length` (`self.OverlappedT1Units`)) (`KismetArrayLibrary.Array_Length` (`self.OverlappedT2Units`)))
    (set `self.Team` 0)
    (`self.SetFlagColor`)
    (`self.CheckOwnedBuilding` 0)))

(event `self.Control Zone.OnComponentBeginOverlap`
  (params (OverlappedComponent :type "PrimitiveComponent Object Reference") (OtherActor :type "Actor Object Reference") (OtherComp :type "PrimitiveComponent Object Reference") (OtherBodyIndex :type Integer) (bFromSweep :type Boolean) (SweepResult :type "HitResult Structure (by ref)"))
  (`/Engine/EditorBlueprintResources/ActorMacros.Switch Has Authority`
    (:`Authority`
      (bind _asbase_unit (cast `BaseUnit` OtherActor))
      (if (== (`self.Team`) -1)
        (bind _team (`BaseUnit.Team` _asbase_unit))
        (set `self.Team` _team)
        (`self.SetFlagColor`)
        (`self.CheckOwnedBuilding` _team))
      (switch `int` _team
        (:`0`
          (`KismetArrayLibrary.Array_Add` (`self.OverlappedT1Units`) _asbase_unit))
        (:`1`
          (`KismetArrayLibrary.Array_Add` (`self.OverlappedT2Units`) _asbase_unit))))))

(event `self.ReceiveTick`
  (params (DeltaSeconds :type "Float (single-precision)"))
  (`/Engine/EditorBlueprintResources/ActorMacros.Switch Has Authority`
    (:`Authority`
      (switch `int` (`self.Team`)
        (:`0`
          (`self.CheckTeam1`))
        (:`1`
          (`self.CheckTeam2`))))))

(event `self.Control Zone.OnComponentEndOverlap`
  (params (OverlappedComponent :type "PrimitiveComponent Object Reference") (OtherActor :type "Actor Object Reference") (OtherComp :type "PrimitiveComponent Object Reference") (OtherBodyIndex :type Integer))
  (`/Engine/EditorBlueprintResources/ActorMacros.Switch Has Authority`
    (:`Authority`
      (bind _asbase_unit (cast `BaseUnit` OtherActor))
      (switch `int` (`BaseUnit.Team` _asbase_unit)
        (:`0`
          (`KismetArrayLibrary.Array_RemoveItem` (`self.OverlappedT1Units`) _asbase_unit))
        (:`1`
          (`KismetArrayLibrary.Array_RemoveItem` (`self.OverlappedT2Units`) _asbase_unit))))))

(event `CheckOwnedBuilding`
  (params (newTeam :type Integer))
  (bind _controlledbuilding (`self.ControlledBuilding`))
  (`/Engine/EditorBlueprintResources/StandardMacros.IsValid` _controlledbuilding
    (:`Is Valid`
      (if (`/Game/GameFiles/TESTING/Blueprints/Buildings/Demo_UnitSpawner.bActive` _controlledbuilding)
        (set `BaseBuilding.Team` newTeam _controlledbuilding)
        (else
          (set `/Game/GameFiles/TESTING/Blueprints/Buildings/Demo_UnitSpawner.bActive` true _controlledbuilding)
          (set `BaseBuilding.Team` newTeam _controlledbuilding)
          (`/Game/GameFiles/TESTING/Blueprints/Buildings/Demo_UnitSpawner.SpawnUnitsTimer` _controlledbuilding))))))

(event `RemoveFromObj`
  (params (Unit :type "BaseUnit Object Reference") (Team :type Integer))
  (bind _overlappedt2units (`self.OverlappedT2Units`))
  (bind _overlappedt1units (`self.OverlappedT1Units`))
  (bind _returnvalue (`KismetArrayLibrary.Array_Find` _overlappedt1units))
  (bind _returnvalue_2 (`KismetArrayLibrary.Array_Find` _overlappedt2units))
  (if (!= Unit null)
    (switch `int` Team
      (:`0`
        (if (!= _returnvalue -1)
          (`KismetArrayLibrary.Array_Remove` _overlappedt1units _returnvalue)))
      (:`1`
        (if (!= _returnvalue_2 -1)
          (`KismetArrayLibrary.Array_Remove` _overlappedt2units _returnvalue_2))))))

(fn `OnRep_Team`
  (`self.SetFlagColor`))

(fn `UserConstructionScript`)