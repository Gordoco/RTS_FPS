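; Demo map match handler that decides a winning team and ends the game.
; On BeginPlay only, it tests both dead counters against a threshold, then queries the RTS_FPSGameInstance for either team having no units left.
; Win clears the game instance's unit tracker, sends every RTS_FPSController a team win screen with disconnect, then destroys the handler.
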(event `self.ReceiveBeginPlay`
  (if (>= (`self.NumDeadT1`) 100)
    (`self.Win` 1)
    (elif (>= (`self.NumDeadT2`) 100)
      (`self.Win` 2)
      (else
        (bind _asrts_fpsgame_instance (cast `RTS_FPSGameInstance` (`GameplayStatics.GetGameInstance`)))
        (bind _returnvalue (`RTS_FPSGameInstance.GetNumberOfUnitsTeam` _asrts_fpsgame_instance 0))
        (bind _returnvalue_2 (`RTS_FPSGameInstance.GetNumberOfUnitsTeam` _asrts_fpsgame_instance 1))
        (if (<= _returnvalue 0)
          (`self.Win` 1)
          (elif (<= _returnvalue_2 0)
            (`self.Win` 2)))))))

(fn `UserConstructionScript`)

(fn `Win`
  (params (WinningTeam :type Integer))
  (bind _asrts_fpsgame_instance (cast `RTS_FPSGameInstance` (`GameplayStatics.GetGameInstance`))
    (:`then`
      (`RTS_FPSGameInstance.ClearUnitTracker` _asrts_fpsgame_instance))
    (:`CastFailed`
      _))
  (bind _outactors (`GameplayStatics.GetAllActorsOfClass` "/Game/GameFiles/Blueprints/Players/Controllers/RTS_FPSController.RTS_FPSController_C"))
  (for _array_element _outactors
    (`/Game/GameFiles/Blueprints/Players/Controllers/RTS_FPSController.Client_WinScreenAndDisconnect` _array_element (`KismetStringLibrary.Concat_StrStr` "Team: " (`KismetStringLibrary.Conv_IntToString` WinningTeam) " Wins!")))
  (`self.K2_DestroyActor`))