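; DemoMapHandler is an actor that decides the winner of a demo map by checking team ownership of ConquestObj objectives.
; It caches all objectives at BeginPlay, then a looping timer tallies how many each team holds.
; When one team holds all of them, Win clears the game instance's unit tracker, calls each RTS_FPSController to show the win screen and disconnect, then destroys the handler.
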(event `self.ReceiveBeginPlay`
  (bind _outactors (`GameplayStatics.GetAllActorsOfClass` "/Game/GameFiles/TESTING/Blueprints/Misc/ConquestObj.ConquestObj_C"))
  (set `self.Objs` _outactors)
  (`KismetSystemLibrary.K2_SetTimerDelegate` (delegate `CheckForWinner`) 1.0 true))

(event `CheckForWinner`
  (for _array_element (`self.Objs`)
    (switch `int` (`/Game/GameFiles/TESTING/Blueprints/Misc/ConquestObj.Team` _array_element)
      (:`0`
        (`/Engine/EditorBlueprintResources/StandardMacros.IncrementInt` (`self.Team1Num`)))
      (:`1`
        (`/Engine/EditorBlueprintResources/StandardMacros.IncrementInt` (`self.Team2Num`)))))
  (if (== (`self.Team1Num`) (`KismetArrayLibrary.Array_Length` (`self.Objs`)))
    (`self.Win` 1)
    (elif (== (`self.Team2Num`) (`KismetArrayLibrary.Array_Length` (`self.Objs`)))
      (`self.Win` 2)
      (else
        (set `self.Team1Num` 0)
        (set `self.Team2Num` 0)))))

(fn `UserConstructionScript`)

(fn `Win`
  (params (WinningTeam :type Integer))
  (locals (OutText :type String))
  (bind _asrts_fpsgame_instance (cast `RTS_FPSGameInstance` (`GameplayStatics.GetGameInstance`))
    (:`then`
      (`RTS_FPSGameInstance.ClearUnitTracker` _asrts_fpsgame_instance))
    (:`CastFailed`
      _))
  (bind _outactors (`GameplayStatics.GetAllActorsOfClass` "/Game/GameFiles/Blueprints/Players/Controllers/RTS_FPSController.RTS_FPSController_C"))
  (for _array_element _outactors
    (`/Game/GameFiles/Blueprints/Players/Controllers/RTS_FPSController.Client_WinScreenAndDisconnect` _array_element (`KismetStringLibrary.Concat_StrStr` "Team: " (`KismetStringLibrary.Conv_IntToString` WinningTeam) " Wins!")))
  (`self.K2_DestroyActor`))