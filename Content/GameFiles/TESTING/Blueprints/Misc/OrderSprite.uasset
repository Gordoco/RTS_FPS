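; OrderSprite is an order marker actor that hovers over a target Enemy and faces its OwningPlayer.
; Each Tick it teleports above the enemy by its capsule half-height, or stays put without a valid enemy, then turns toward the player with a 90-degree yaw offset.
; It destroys itself when the owner is invalid or dead, the enemy dies, or the owner overlaps its Collision, including at BeginPlay.
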(event `self.ReceiveBeginPlay`
  (for _array_element (`PrimitiveComponent.GetOverlappingActors` (`self.Collision`) "/Script/RTS_FPS.FPSCharacter")
    (if (== (`self.OwningPlayer`) _array_element)
      (`self.K2_DestroyActor`))))

(event `self.ReceiveTick`
  (params (DeltaSeconds :type "Float (single-precision)"))
  (`self.TeleportToEnemy`)
  (`self.RotateToFace`))

(event `RotateToFace`
  (`self.K2_SetActorRotation` (`KismetMathLibrary.MakeRotator` (.roll (`KismetMathLibrary.FindLookAtRotation` (`self.K2_GetActorLocation`) (`self.K2_GetActorLocation` (`self.OwningPlayer`)))) (.pitch (`KismetMathLibrary.FindLookAtRotation` (`self.K2_GetActorLocation`) (`self.K2_GetActorLocation` (`self.OwningPlayer`)))) (+ (.yaw (`KismetMathLibrary.FindLookAtRotation` (`self.K2_GetActorLocation`) (`self.K2_GetActorLocation` (`self.OwningPlayer`)))) 90.0))))

(event `TeleportToEnemy`
  (bind _owningplayer (`self.OwningPlayer`))
  (bind _enemy (`self.Enemy`))
  (`/Engine/EditorBlueprintResources/StandardMacros.IsValid` _owningplayer
    (:`Is Valid`
      (bind _returnvalue (`BaseUnit.IsDead` _owningplayer))
      (if _returnvalue
        (`self.K2_DestroyActor` :!label _label)
        (else
          (`/Engine/EditorBlueprintResources/StandardMacros.IsValid` _enemy
            (:`Is Valid`
              (bind _returnvalue_2 (`BaseUnit.IsDead` _enemy))
              (if _returnvalue_2
                (goto _label)
                (else
                  (`self.K2_SetActorLocation` (`KismetMathLibrary.MakeVector` (.x (`self.K2_GetActorLocation` _enemy)) (.y (`self.K2_GetActorLocation` _enemy)) (+ (.z (`self.K2_GetActorLocation` _enemy)) (`CapsuleComponent.GetScaledCapsuleHalfHeight` (`Character.CapsuleComponent` _enemy)))) false true))))))))
    (:`Is Not Valid`
      (goto _label))))

(event `self.Collision.OnComponentBeginOverlap`
  (params (OverlappedComponent :type "PrimitiveComponent Object Reference") (OtherActor :type "Actor Object Reference") (OtherComp :type "PrimitiveComponent Object Reference") (OtherBodyIndex :type Integer) (bFromSweep :type Boolean) (SweepResult :type "HitResult Structure (by ref)"))
  (if (== (`self.OwningPlayer`) OtherActor)
    (`self.K2_DestroyActor`)))

(fn `UserConstructionScript`)